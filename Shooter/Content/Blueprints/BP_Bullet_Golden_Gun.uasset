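; BP_Bullet_Golden_Gun is a homing bullet projectile that locks onto an enemy when it spawns.
; On BeginPlay it searches actors implementing BPI_Enemy_Hit and homes on the capsule of the last one found within ClosestDistance, which is never updated, so not necessarily the nearest.
; Hits on enemies send damage through the interface with a flesh sound; other hits spawn smoke and a fading bullet-hole decal, and either destroys the bullet.
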(event `self.Bullet.OnComponentHit`
  (params (HitComponent :type "PrimitiveComponent Object Reference") (OtherActor :type "Actor Object Reference") (OtherComp :type "PrimitiveComponent Object Reference") (NormalImpulse :type "Vector Structure") (Hit :type "HitResult Structure (by ref)"))
  (bind (_bblockinghit _binitialoverlap _time _distance _location _impactpoint _normal) (`GameplayStatics.BreakHitResult` Hit))
  (bind (_returnvalue_roll _returnvalue_pitch _returnvalue_yaw) (`KismetMathLibrary.BreakRotator` (`KismetMathLibrary.Conv_VectorToRotator` _normal)))
  ;[1 1 1] Check if enemy
  (if (`KismetSystemLibrary.DoesImplementInterface` OtherActor "/Game/Blueprints/BPI_Enemy_Hit.BPI_Enemy_Hit_C")
    ;[1 1 1] Enemy Hit
    (message `/Game/Blueprints/BPI_Enemy_Hit.Enemy Hit` OtherActor _location (`self.Damage`))
    (`GameplayStatics.PlaySoundAtLocation` "/Game/Sounds/SC_Bullet_Impact_Flesh.SC_Bullet_Impact_Flesh" _location (struct) 1.0 1.0 0.0 null null null null)
    (`self.K2_DestroyActor`)
    (else
      ;[1 1 1] Object Hit Effects
      (`NiagaraFunctionLibrary.SpawnSystemAtLocation` "/Game/VFX/Niagara/NS_Impact_Smoke.NS_Impact_Smoke" _location)
      (bind _returnvalue (`GameplayStatics.SpawnDecalAtLocation` "/Game/Materials/MAT_Bullet_Hole.MAT_Bullet_Hole" (10.0 20.0 20.0) _location (`KismetMathLibrary.MakeRotator` (`KismetMathLibrary.RandomFloatInRange` 0.0 360.0) _returnvalue_pitch _returnvalue_yaw) 3.0))
      (`DecalComponent.SetFadeScreenSize` _returnvalue 0.005)
      (`DecalComponent.SetFadeOut` _returnvalue 0.5 2.5 true)
      (`self.K2_DestroyActor`))))

(event `Lock On`
  (bind _projectilemovement (`self.ProjectileMovement`))
  (bind _homing_target (`self.FindHomingTarget`))
  (set `ProjectileMovementComponent.HomingTargetComponent` _homing_target _projectilemovement)
  (set `ProjectileMovementComponent.bIsHomingProjectile` true _projectilemovement))

(event `self.ReceiveBeginPlay`
  (`self.Lock On`))

(fn `FindHomingTarget`
  (returns (`Homing Target` :type "SceneComponent Object Reference"))
  (bind _outactors (`GameplayStatics.GetAllActorsWithInterface` "/Game/Blueprints/BPI_Enemy_Hit.BPI_Enemy_Hit_C"))
  (if (not (== (`KismetArrayLibrary.Array_Length` _outactors) 0))
    (for _array_element _outactors
      (if (< (`KismetMathLibrary.VSize` (`KismetMathLibrary.Vector_GetAbs` (- (`self.K2_GetActorLocation` _array_element) (`self.K2_GetActorLocation`)))) (`self.Closest Distance`))
        (set `self.Homing Target` _array_element)))
    (return (`self.GetComponentByClass` (`self.Homing Target`) "/Script/Engine.CapsuleComponent"))))

(fn `UserConstructionScript`)