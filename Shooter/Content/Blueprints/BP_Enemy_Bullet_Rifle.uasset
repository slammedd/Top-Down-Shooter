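; Enemy rifle bullet that damages the player or leaves an impact effect on whatever else it hits.
; On component hit, it sends damage and hit location to actors implementing BPI_Player_Hit.
; Other hits spawn Niagara impact smoke and a fading bullet hole decal aligned to the surface normal with random roll.
; The bullet destroys itself after either outcome.
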(event `self.Bullet.OnComponentHit`
  (params (HitComponent :type "PrimitiveComponent Object Reference") (OtherActor :type "Actor Object Reference") (OtherComp :type "PrimitiveComponent Object Reference") (NormalImpulse :type "Vector Structure") (Hit :type "HitResult Structure (by ref)"))
  (bind (_bblockinghit _binitialoverlap _time _distance _location _impactpoint _normal) (`GameplayStatics.BreakHitResult` Hit))
  (bind (_returnvalue_roll _returnvalue_pitch _returnvalue_yaw) (`KismetMathLibrary.BreakRotator` (`KismetMathLibrary.Conv_VectorToRotator` _normal)))
  (if (`KismetSystemLibrary.DoesImplementInterface` OtherActor "/Game/Blueprints/BPI_Player_Hit.BPI_Player_Hit_C")
    (message `/Game/Blueprints/BPI_Player_Hit.Player Hit` OtherActor (`self.Damage`) _location)
    (`self.K2_DestroyActor`)
    (else
      (`NiagaraFunctionLibrary.SpawnSystemAtLocation` "/Game/VFX/Niagara/NS_Impact_Smoke.NS_Impact_Smoke" _location)
      (bind _returnvalue (`GameplayStatics.SpawnDecalAtLocation` "/Game/Materials/MAT_Bullet_Hole.MAT_Bullet_Hole" (10.0 20.0 20.0) _location (`KismetMathLibrary.MakeRotator` (`KismetMathLibrary.RandomFloatInRange` 0.0 360.0) _returnvalue_pitch _returnvalue_yaw) 3.0))
      (`DecalComponent.SetFadeScreenSize` _returnvalue 0.005)
      (`DecalComponent.SetFadeOut` _returnvalue 0.5 2.5 true)
      (`self.K2_DestroyActor`))))

(fn `UserConstructionScript`)