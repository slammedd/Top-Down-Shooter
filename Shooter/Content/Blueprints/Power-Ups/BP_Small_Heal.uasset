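; Small health pickup that adds a fixed amount to the Health of the BP_ThirdPersonCharacter overlapping its box, without clamping.
; A DoOnce limits it to one use, hiding the mesh, playing pickup sounds and attaching a healing Niagara effect to the character.
; A timer started on BeginPlay destroys the actor after ten seconds with a smoke puff and sound, even if it was already collected.
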(event `self.ReceiveBeginPlay`
  (`self.Auto Destroy`))

(event `Auto Destroy`
  (bind _returnvalue (`self.K2_GetActorLocation`))
  (`KismetSystemLibrary.Delay` 10.0)
  (`NiagaraFunctionLibrary.SpawnSystemAtLocation` "/Game/VFX/Niagara/NS_Death_Smoke.NS_Death_Smoke" _returnvalue)
  (`GameplayStatics.PlaySoundAtLocation` "/Game/Sounds/SC_Smoke_Poof.SC_Smoke_Poof" _returnvalue (struct) 1.0 1.0 0.0 null null null null)
  (`self.K2_DestroyActor`))

(event `self.Box.OnComponentBeginOverlap`
  (params (OverlappedComponent :type "PrimitiveComponent Object Reference") (OtherActor :type "Actor Object Reference") (OtherComp :type "PrimitiveComponent Object Reference") (OtherBodyIndex :type Integer) (bFromSweep :type Boolean) (SweepResult :type "HitResult Structure (by ref)"))
  (bind _returnvalue (`self.K2_GetActorLocation`))
  (bind _asbp_third_person_character (cast `/Game/Blueprints/BP_ThirdPersonCharacter` OtherActor))
  (`/Engine/EditorBlueprintResources/StandardMacros.DoOnce` false
    (:`Completed`
      (`SceneComponent.SetHiddenInGame` (`self.StaticMesh`) true false)
      (`GameplayStatics.PlaySoundAtLocation` "/Game/Sounds/SC_Pickup.SC_Pickup" _returnvalue (struct) 1.0 1.0 0.0 null null null null)
      (`GameplayStatics.PlaySoundAtLocation` "/Game/Sounds/SC_Healing_Pack.SC_Healing_Pack" _returnvalue (struct) 1.0 1.0 0.0 null null null null)
      (set `/Game/Blueprints/BP_ThirdPersonCharacter.Health` (+ (`/Game/Blueprints/BP_ThirdPersonCharacter.Health` _asbp_third_person_character) 20.0) _asbp_third_person_character)
      (`NiagaraFunctionLibrary.SpawnSystemAttached` "/Game/VFX/Niagara/NS_Healing.NS_Healing" (`Character.CapsuleComponent` _asbp_third_person_character) "None" (0.0 0.0 -80.0) (struct) "KeepRelativeOffset" true))))

(fn `UserConstructionScript`)