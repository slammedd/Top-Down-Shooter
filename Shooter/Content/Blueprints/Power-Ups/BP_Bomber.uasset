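; Bomber power-up actor that plays an attached sound and, after a short delay, drops a run of BP_Bomb actors.
; Three looping timers with staggered initial delays spawn bombs at three separate drop-point components.
; Each drop event also starts a Delay that clears its own timer, limiting the bombing run to a few seconds.
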(event `self.ReceiveBeginPlay`
  (`GameplayStatics.SpawnSoundAttached` "/Game/Sounds/SC_Bomber.SC_Bomber" (`self.StaticMesh`) "None" (0.0 0.0 0.0) (struct) "KeepRelativeOffset" false 1.0 1.0 0.0 null null)
  (`KismetSystemLibrary.Delay` 5.5)
  (bind _returnvalue (`KismetSystemLibrary.K2_SetTimerDelegate` (delegate `Drop Bombs`) 0.3 true))
  (bind _returnvalue_2 (`KismetSystemLibrary.K2_SetTimerDelegate` (delegate `Drop Bombs 1`) 0.3 true 0.3))
  (bind _returnvalue_3 (`KismetSystemLibrary.K2_SetTimerDelegate` (delegate `Drop Bombs 2`) 0.3 true 0.6)))

(event `Drop Bombs`
  (`|SpawnActorFromClass` "/Game/Blueprints/Power-Ups/BP_Bomb.BP_Bomb_C" (`KismetMathLibrary.MakeTransform` (`SceneComponent.K2_GetComponentLocation` (`self.Drop Point`))) "Undefined" "OverrideRootScale" null null)
  (`KismetSystemLibrary.Delay` 4.0)
  (`KismetSystemLibrary.K2_ClearAndInvalidateTimerHandle` (stale `self.ReceiveBeginPlay` _returnvalue)))

(event `Drop Bombs 1`
  (`|SpawnActorFromClass` "/Game/Blueprints/Power-Ups/BP_Bomb.BP_Bomb_C" (`KismetMathLibrary.MakeTransform` (`SceneComponent.K2_GetComponentLocation` (`self.Drop Point1`))) "Undefined" "OverrideRootScale" null null)
  (`KismetSystemLibrary.Delay` 4.0)
  (`KismetSystemLibrary.K2_ClearAndInvalidateTimerHandle` (stale `self.ReceiveBeginPlay` _returnvalue_2)))

(event `Drop Bombs 2`
  (`|SpawnActorFromClass` "/Game/Blueprints/Power-Ups/BP_Bomb.BP_Bomb_C" (`KismetMathLibrary.MakeTransform` (`SceneComponent.K2_GetComponentLocation` (`self.Drop Point2`))) "Undefined" "OverrideRootScale" null null)
  (`KismetSystemLibrary.Delay` 4.0)
  (`KismetSystemLibrary.K2_ClearAndInvalidateTimerHandle` (stale `self.ReceiveBeginPlay` _returnvalue_3)))

(fn `UserConstructionScript`)