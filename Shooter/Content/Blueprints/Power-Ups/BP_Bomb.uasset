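; BP_Bomb is a power-up bomb that explodes on impact and damages enemies.
; The mesh's first hit passes a DoOnce and, unless against another BP_Bomb, spawns explosion and dirt effects with sound, then hides the mesh and stops its physics.
; Independently of that hit, Sphere overlaps send heavy damage through BPI_Enemy_Hit to any implementing actor.
; The actor is never destroyed here.
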(event `self.StaticMesh.OnComponentHit`
  (params (HitComponent :type "PrimitiveComponent Object Reference") (OtherActor :type "Actor Object Reference") (OtherComp :type "PrimitiveComponent Object Reference") (NormalImpulse :type "Vector Structure") (Hit :type "HitResult Structure (by ref)"))
  (bind (_bblockinghit _binitialoverlap _time _distance _location) (`GameplayStatics.BreakHitResult` Hit))
  (`/Engine/EditorBlueprintResources/StandardMacros.DoOnce` false
    (:`Completed`
      (cast `/Game/Blueprints/Power-Ups/BP_Bomb` OtherActor
        (:`CastFailed`
          (`NiagaraFunctionLibrary.SpawnSystemAtLocation` "/Game/VFX/Niagara/NS_Explosion.NS_Explosion" _location)
          (`NiagaraFunctionLibrary.SpawnSystemAtLocation` "/Game/VFX/Niagara/NS_Dirt_Particles.NS_Dirt_Particles" _location)
          (`GameplayStatics.PlaySoundAtLocation` "/Game/Sounds/SC_Bomb_Explosion.SC_Bomb_Explosion" _location (struct) 1.0 1.0 0.0 null null null null)
          (`SceneComponent.SetHiddenInGame` (`self.StaticMesh`) true false)
          (`PrimitiveComponent.SetSimulatePhysics` (`self.StaticMesh`) false))))))

(event `self.Sphere.OnComponentBeginOverlap`
  (params (OverlappedComponent :type "PrimitiveComponent Object Reference") (OtherActor :type "Actor Object Reference") (OtherComp :type "PrimitiveComponent Object Reference") (OtherBodyIndex :type Integer) (bFromSweep :type Boolean) (SweepResult :type "HitResult Structure (by ref)"))
  (if (`KismetSystemLibrary.DoesImplementInterface` OtherActor "/Game/Blueprints/BPI_Enemy_Hit.BPI_Enemy_Hit_C")
    (message `/Game/Blueprints/BPI_Enemy_Hit.Enemy Hit` OtherActor (`self.K2_GetActorLocation`) 1000.0)))

(fn `UserConstructionScript`)