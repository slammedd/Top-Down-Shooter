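; BP_Shield_Sphere is a power-up pickup that gives the third-person character a shield sphere.
; On box overlap, if the character holds no power-up, it sets the ShieldSphere power-up, starts a HUD timer, calls SetShieldSphere and destroys itself with a pickup sound.
; A DoOnce gate limits collection to a single trigger.
; If left uncollected, it self-destructs after a short delay with a smoke effect and poof sound.
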(event `self.ReceiveBeginPlay`
  (`self.Auto Destroy`))

(event `Auto Destroy`
  (bind _returnvalue (`self.K2_GetActorLocation`))
  (`KismetSystemLibrary.Delay` 10.0)
  (`NiagaraFunctionLibrary.SpawnSystemAtLocation` "/Game/VFX/Niagara/NS_Death_Smoke.NS_Death_Smoke" _returnvalue)
  (`GameplayStatics.PlaySoundAtLocation` "/Game/Sounds/SC_Smoke_Poof.SC_Smoke_Poof" _returnvalue (struct) 1.0 1.0 0.0 null null null null)
  (`self.K2_DestroyActor`))

(event `self.Box.OnComponentBeginOverlap`
  (params (OverlappedComponent :type "PrimitiveComponent Object Reference") (OtherActor :type "Actor Object Reference") (OtherComp :type "PrimitiveComponent Object Reference") (OtherBodyIndex :type Integer) (bFromSweep :type Boolean) (SweepResult :type "HitResult Structure (by ref)"))
  (bind _asbp_third_person_character (cast `/Game/Blueprints/BP_ThirdPersonCharacter` OtherActor))
  (switch `/Game/Blueprints/Power-Ups/ENUM_Power_Ups` (`/Game/Blueprints/BP_ThirdPersonCharacter.Power Up` _asbp_third_person_character)
    (:`NewEnumerator0`
      (`/Engine/EditorBlueprintResources/StandardMacros.DoOnce` false
        (:`Completed`
          (`GameplayStatics.PlaySoundAtLocation` "/Game/Sounds/SC_Pickup.SC_Pickup" (`self.K2_GetActorLocation`) (struct) 1.0 1.0 0.0 null null null null)
          (set `/Game/Blueprints/BP_ThirdPersonCharacter.Power Up` "NewEnumerator5" _asbp_third_person_character)
          (`/Game/UI/WB_Player_HUD.Start Power Up Timer` (`/Game/Blueprints/BP_ThirdPersonCharacter.HUD` _asbp_third_person_character) 15)
          (`/Game/Blueprints/BP_ThirdPersonCharacter.Set Shield Sphere` _asbp_third_person_character)
          (`self.K2_DestroyActor`))))))

(fn `UserConstructionScript`)