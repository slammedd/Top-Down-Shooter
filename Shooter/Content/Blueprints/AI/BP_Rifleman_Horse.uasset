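; Rifleman enemy character (horse variant) that runs BT_Rifleman_Horse and shoots at the player.
; Tick starts the firing montage while it moves with the blackboard reporting the player in range, otherwise stopping it.
; FireWeapon spawns bullets aimed ahead of the player using velocity and distance.
; EnemyHit applies damage with material flash and flinch, then on death counts the kill, ragdolls, puffs smoke and may drop a heal.
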(event `Stop Firing`
  ;[1 1 1] Start/Stop Firing
  (`self.StopAnimMontage` "/Game/Animations/AM_Shoot_Rifleman.AM_Shoot_Rifleman")
  (`self.StopAnimMontage` "/Game/Animations/AM_Shoot_Standing.AM_Shoot_Standing")
  (set `self.Is Shooting` false))

(event `Start Firing`
  ;[1 1 1] Start/Stop Firing
  (if (not (`self.Is Shooting`))
    (set `self.Is Shooting` true)
    (`self.PlayAnimMontage` "/Game/Animations/AM_Shoot_Rifleman.AM_Shoot_Rifleman" (`self.Fire Rate`))))

(event `Fire Weapon`
  (bind _returnvalue (`GameplayStatics.GetPlayerCharacter` 0))
  (bind _muzzle_flash (`self.Muzzle Flash`))
  (bind _returnvalue_2 (`SceneComponent.K2_GetComponentLocation` (`self.Spawner`)))
  ;[1 1 1] Spawn Bullet
  (if (`self.Can Shoot`)
    (bind _returnvalue_3 (`|SpawnActorFromClass` "/Game/Blueprints/BP_Enemy_Bullet_Rifle.BP_Enemy_Bullet_Rifle_C" (`KismetMathLibrary.MakeTransform` _returnvalue_2 (`KismetMathLibrary.FindLookAtRotation` _returnvalue_2 (+ (+ (`SceneComponent.K2_GetComponentLocation` (`Character.CapsuleComponent` _returnvalue)) (0.0 0.0 0.0)) (* (`self.GetVelocity` _returnvalue) (/ (`self.GetDistanceTo` self _returnvalue) (* (`self.Bullet Speed`) 5.0))))) (0.194709 0.032197 0.032197)) "Undefined" "OverrideRootScale" null null))
    (bind _projectilemovement (`/Game/Blueprints/BP_Enemy_Bullet_Rifle.ProjectileMovement` _returnvalue_3))
    (set `MovementComponent.Velocity` (* (`MovementComponent.Velocity` _projectilemovement) (`self.Bullet Speed`)) _projectilemovement)
    ;[1 1 1] Trigger Muzzle Flash
    (`GameplayStatics.PlaySoundAtLocation` "/Game/Sounds/SC_Rifle_Shot.SC_Rifle_Shot" (`self.K2_GetActorLocation`) (struct) 1.0 1.0 0.0 null null null null)
    (`ActorComponent.Activate` _muzzle_flash false)
    (`KismetSystemLibrary.Delay` 0.3)
    (`ActorComponent.Deactivate` _muzzle_flash)))

(event `self.ReceiveTick`
  (params (DeltaSeconds :type "Float (single-precision)"))
  (bind _returnvalue (`GameplayStatics.GetPlayerCharacter` 0))
  (set `self.Predicted Rotation` (`KismetMathLibrary.FindLookAtRotation` (`SceneComponent.K2_GetComponentLocation` (`self.Spawner`)) (+ (+ (`SceneComponent.K2_GetComponentLocation` (`Character.CapsuleComponent` _returnvalue)) (0.0 0.0 0.0)) (* (`self.GetVelocity` _returnvalue) (/ (`self.GetDistanceTo` self _returnvalue) (* (`self.Bullet Speed`) 5.0))))))
  (if (`self.Is Dead`)
    _
    (elif (not (`self.Player Died`))
      ;[1 1 1] AI Shooting Animation Control
      (if (> (`KismetMathLibrary.VSize` (`self.GetVelocity`)) 150.0)
        (if (`BlackboardComponent.GetValueAsBool` (`AIBlueprintHelperLibrary.GetBlackboard` null) "Player In Range")
          (`self.Start Firing`)
          (goto _label :!via `Reset`)
          (else
            (`self.Stop Firing`)))
        (else
          (`/Engine/EditorBlueprintResources/StandardMacros.DoOnce` false :!label _label
            (:`Completed`
              (`self.Stop Firing`))))))))

(event `Revert Hit Material`
  ;[1 1 1] Revert Hit Material
  (`KismetSystemLibrary.Delay` 0.075)
  (`PrimitiveComponent.SetMaterial` (`self.Mesh`) 0 "/Game/StylizedArmyPackA/materials/M_soldier_body_germany.M_soldier_body_germany")
  (`PrimitiveComponent.SetMaterial` (`self.Default Rifle`) 0 "/Game/StylizedArmyPackA/materials/M_mouse_rifle.M_mouse_rifle")
  (`PrimitiveComponent.SetMaterial` (`self.Backpack`) 0 "/Game/StylizedArmyPackA/materials/M_soldier_backpack_germany.M_soldier_backpack_germany")
  (`PrimitiveComponent.SetMaterial` (`self.Hat`) 0 "/Game/StylizedArmyPackA/materials/M_soldier_cap_russia.M_soldier_cap_russia"))

(event `Death Effect`
  (bind _mesh (`self.Mesh`))
  ;[1 1 1] Death Smoke
  (`KismetSystemLibrary.Delay` 0.2)
  (`PrimitiveComponent.SetCollisionEnabled` (`self.CapsuleComponent`) "NoCollision")
  (`PrimitiveComponent.SetCollisionProfileName` _mesh "Ragdoll" true)
  (`PrimitiveComponent.SetSimulatePhysics` _mesh true)
  (`PrimitiveComponent.AddImpulse` _mesh (0.0 0.0 500.0) "None" false)
  (`CharacterMovementComponent.DisableMovement` (`self.CharacterMovement`))
  (`KismetSystemLibrary.PrintString` "Rifleman Dead")
  (`KismetSystemLibrary.Delay` 3.5)
  (`GameplayStatics.PlaySoundAtLocation` "/Game/Sounds/SC_Smoke_Poof.SC_Smoke_Poof" (`self.K2_GetActorLocation`) (struct) 1.0 1.0 0.0 null null null null)
  (`ActorComponent.Activate` (`self.NS_Death_Smoke`) false)
  (`KismetSystemLibrary.Delay` 0.3)
  (`SceneComponent.SetHiddenInGame` (`self.Mesh`) true true)
  (`self.Stop Firing`)
  (`KismetSystemLibrary.Delay` 1.0)
  (`self.K2_DestroyActor`))

(event `self.ReceiveBeginPlay`
  ;[1 1 1] Face Player on Spawn
  (`self.K2_SetActorRotation` (`KismetMathLibrary.FindLookAtRotation` (`self.K2_GetActorLocation`) (`SceneComponent.K2_GetComponentLocation` (`Character.CapsuleComponent` (`GameplayStatics.GetPlayerCharacter` 0)))))
  (bind _asaicontroller (cast `AIController` (`self.GetController`)))
  (`AIController.RunBehaviorTree` _asaicontroller "/Game/Blueprints/AI/BT_Rifleman_Horse.BT_Rifleman_Horse")
  (bind _asbp_third_person_character (cast `/Game/Blueprints/BP_ThirdPersonCharacter` (`GameplayStatics.GetPlayerCharacter` 0)))
  (set `self.Player` _asbp_third_person_character))

(event `Reset Firing After Hit`
  ;[1 1 1] Reset Firing After Hit
  (if (`self.Is Shooting`)
    (if (not (`self.Is Dead`))
      (`KismetSystemLibrary.Delay` 1.0)
      (`self.PlayAnimMontage` "/Game/Animations/AM_Shoot_Rifleman.AM_Shoot_Rifleman" (`self.Fire Rate`)))))

(event `/Game/Blueprints/BPI_Enemy_Hit.Enemy Hit`
  (params (`Hit Location` :type "Vector Structure") (Damage :type "Float (double-precision)"))
  (bind _mesh (`self.Mesh`))
  ;[1 1 1] Enemy Hit
  (`PrimitiveComponent.SetMaterial` (`self.Mesh`) 0 "/Game/Materials/MAT_Enemy_Impact_Inst.MAT_Enemy_Impact_Inst")
  (`PrimitiveComponent.SetMaterial` (`self.Default Rifle`) 0 "/Game/Materials/MAT_Enemy_Impact_Inst.MAT_Enemy_Impact_Inst")
  (`PrimitiveComponent.SetMaterial` (`self.Backpack`) 0 "/Game/Materials/MAT_Enemy_Impact_Inst.MAT_Enemy_Impact_Inst")
  (`PrimitiveComponent.SetMaterial` (`self.Hat`) 0 "/Game/Materials/MAT_Enemy_Impact_Inst.MAT_Enemy_Impact_Inst")
  (`NiagaraFunctionLibrary.SpawnSystemAtLocation` "/Game/VFX/Niagara/NS_Hit_Impact.NS_Hit_Impact" `Hit Location`)
  (set `self.Health` (- (`self.Health`) Damage))
  (if (== (`KismetMathLibrary.RandomIntegerInRange` 0 1) 0)
    (`self.PlayAnimMontage` "/Game/Animations/AM_Damage1.AM_Damage1" 1.5)
    (else
      (`self.PlayAnimMontage` "/Game/Animations/AM_Damage2.AM_Damage2" 1.5)))
  (`self.Revert Hit Material`)
  (`self.Reset Firing After Hit`)
  ;[1 1 1] Death
  (if (<= (`self.Health`) 0.0)
    (if (not (`self.Is Dead`))
      (`/Engine/EditorBlueprintResources/StandardMacros.IncrementInt` (`/Game/Blueprints/BP_ThirdPersonCharacter.Enemies Killed` (`self.Player`))
        (:`  `
          (`self.Stop Firing`)
          (set `self.Is Dead` true)
          (set `self.Can Shoot` false)
          (`BlackboardComponent.SetValueAsBool` (`AIBlueprintHelperLibrary.GetBlackboard` null) "Is Dead" true)
          (`self.StopAnimMontage` "/Game/Animations/AM_Shoot_Rifleman.AM_Shoot_Rifleman")
          (`CharacterMovementComponent.DisableMovement` (`self.CharacterMovement`))
          (`GameplayStatics.PlaySoundAtLocation` "/Game/Sounds/SC_Enemy_Die.SC_Enemy_Die" `Hit Location` (struct) 1.0 1.0 0.0 null null null null)
          (`PrimitiveComponent.SetCollisionEnabled` (`self.CapsuleComponent`) "NoCollision")
          (`KismetSystemLibrary.Delay` 0.3)
          (`PrimitiveComponent.SetCollisionProfileName` _mesh "Ragdoll" true)
          (`PrimitiveComponent.SetSimulatePhysics` _mesh true)
          (`PrimitiveComponent.AddImpulse` _mesh (0.0 0.0 500.0) "None" false)
          (`KismetSystemLibrary.PrintString` "Rifleman Dead")
          (`KismetSystemLibrary.Delay` 3.5)
          (`GameplayStatics.PlaySoundAtLocation` "/Game/Sounds/SC_Smoke_Poof.SC_Smoke_Poof" (`self.K2_GetActorLocation`) (struct) 1.0 1.0 0.0 null null null null)
          (`ActorComponent.Activate` (`self.NS_Death_Smoke`) false)
          (`self.Chance to Drop Heal`)
          (`KismetSystemLibrary.Delay` 0.3)
          (`SceneComponent.SetHiddenInGame` (`self.Mesh`) true true)
          (`KismetSystemLibrary.Delay` 1.0)
          (`self.K2_DestroyActor`))))))

(event `Chance to Drop Heal`
  (if (== (`KismetMathLibrary.RandomIntegerInRange` 0 3) 0)
    (`|SpawnActorFromClass` "/Game/Blueprints/Power-Ups/BP_Small_Heal.BP_Small_Heal_C" (`KismetMathLibrary.MakeTransform` (`SceneComponent.K2_GetComponentLocation` (`self.Mesh`))) "Undefined" "OverrideRootScale" null null)))

(event `/Game/Blueprints/BPI_Enemy_Hit.Player Dead`
  ;[1 1 1] Player Dead
  (set `self.Player Died` true)
  (`self.Stop Firing`)
  (`CharacterMovementComponent.DisableMovement` (`self.CharacterMovement`)))

(fn `UserConstructionScript`)