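; Flamethrower enemy AI character that fires when the Blackboard flags the player in range and it is nearly stationary.
; A timeline extends a box trace from the spawner, starting damage on the player and randomly igniting them.
; AI perception updates sight in the Blackboard; hits flash materials and briefly interrupt firing, while death ragdolls, smokes and destroys the actor.
; Also retains rifleman-style FireWeapon logic that leads shots using player velocity.
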(event `Stop Firing`
  (bind _spawner (`self.Spawner`))
  (bind _returnvalue (`SceneComponent.K2_GetComponentLocation` _spawner))
  ;[1 1 1] Start/Stop Firing
  (if (`self.Is Shooting`)
    (set `self.Is Shooting` false)
    (`AudioComponent.FadeOut` (`self.Flamethrower Sound`) 0.25 0.0 "Linear")
    (bind _asbp_third_person_character (cast `/Game/Blueprints/BP_ThirdPersonCharacter` (`GameplayStatics.GetPlayerCharacter` 0)))
    (`/Game/Blueprints/BP_ThirdPersonCharacter.Stop Flamethrower Damage` _asbp_third_person_character)
    (`ActorComponent.Deactivate` (`self.Flamethrower`))
    (bind (_direction _box) (`Timeline|Box Trace` :!via `Stop` :!label _label)
      (:`Update`
        (bind (_outhit _returnvalue_2) (`KismetSystemLibrary.BoxTraceSingleByProfile` :`Start` _returnvalue :`End` (+ _returnvalue (* (`SceneComponent.GetForwardVector` _spawner) _box)) :`HalfSize` (50.0 50.0 10.0) :`ProfileName` "Pawn" :`DrawTime` 1.0))
        (if _returnvalue_2
          (bind _asbp_third_person_character_2 (cast `/Game/Blueprints/BP_ThirdPersonCharacter` (`.HitActor` (`GameplayStatics.BreakHitResult` _outhit))))
          (if (== (`KismetMathLibrary.RandomIntegerInRange` 1 10) 5)
            (`/Game/Blueprints/BP_ThirdPersonCharacter.Activate Fire` _asbp_third_person_character_2))
          (`/Engine/EditorBlueprintResources/StandardMacros.DoOnce` false :!label _label_2
            (:`Completed`
              (`/Game/Blueprints/BP_ThirdPersonCharacter.Start Flamethrower Damage` _asbp_third_person_character_2 5.0)))
          (else
            (bind _asbp_third_person_character_3 (cast `/Game/Blueprints/BP_ThirdPersonCharacter` (`GameplayStatics.GetPlayerCharacter` 0)))
            (`/Game/Blueprints/BP_ThirdPersonCharacter.Stop Flamethrower Damage` _asbp_third_person_character_3)
            (goto _label_2 :!via `Reset`))))
      (:`Finished`
        (`self.Stop Firing`)))))

(event `Start Firing`
  ;[1 1 1] Start/Stop Firing
  (if (not (`self.Is Shooting`))
    (set `self.Is Shooting` true)
    (bind _returnvalue (`GameplayStatics.SpawnSoundAttached` "/Game/Sounds/SC_Flamethrower.SC_Flamethrower" (`self.Mesh`) "None" (0.0 0.0 0.0) (struct) "KeepRelativeOffset" false 1.0 1.0 0.0 null null))
    (set `self.Flamethrower Sound` _returnvalue)
    (`ActorComponent.Activate` (`self.Flamethrower`) false)
    (goto _label :!via `PlayFromStart`)))

(event `Fire Weapon`
  (bind _returnvalue (`GameplayStatics.GetPlayerCharacter` 0))
  (bind _returnvalue_2 (`SceneComponent.K2_GetComponentLocation` (`self.Spawner`)))
  ;[1 1 1] Spawn Bullet
  (if (`self.Can Shoot`)
    (bind _returnvalue_3 (`|SpawnActorFromClass` "/Game/Blueprints/BP_Enemy_Bullet_Rifle.BP_Enemy_Bullet_Rifle_C" (`KismetMathLibrary.MakeTransform` _returnvalue_2 (`KismetMathLibrary.FindLookAtRotation` _returnvalue_2 (+ (+ (`SceneComponent.K2_GetComponentLocation` (`Character.CapsuleComponent` _returnvalue)) (0.0 0.0 0.0)) (* (`self.GetVelocity` _returnvalue) (/ (`self.GetDistanceTo` self _returnvalue) (* (`self.Bullet Speed`) 5.0))))) (0.194709 0.032197 0.032197)) "Undefined" "OverrideRootScale" null null))
    (bind _projectilemovement (`/Game/Blueprints/BP_Enemy_Bullet_Rifle.ProjectileMovement` _returnvalue_3))
    (set `MovementComponent.Velocity` (* (`MovementComponent.Velocity` _projectilemovement) (`self.Bullet Speed`)) _projectilemovement)))

(event `self.ReceiveTick`
  (params (DeltaSeconds :type "Float (single-precision)"))
  (bind _returnvalue (`GameplayStatics.GetPlayerCharacter` 0))
  (set `self.Predicted Rotation` (`KismetMathLibrary.FindLookAtRotation` (`SceneComponent.K2_GetComponentLocation` (`self.Spawner`)) (+ (+ (`SceneComponent.K2_GetComponentLocation` (`Character.CapsuleComponent` _returnvalue)) (0.0 0.0 0.0)) (* (`self.GetVelocity` _returnvalue) (/ (`self.GetDistanceTo` self _returnvalue) (* (`self.Bullet Speed`) 5.0))))))
  (if (`self.Is Dead`)
    _
    (elif (`self.Player Died`)
      _
      (elif (`BlackboardComponent.GetValueAsBool` (`AIBlueprintHelperLibrary.GetBlackboard` null) "Player In Range")
        (if (<= (`KismetMathLibrary.VSize` (`self.GetVelocity`)) 1.0)
          (`self.Start Firing`))
        (else
          (`self.Stop Firing`))))))

(event `Revert Hit Material`
  ;[1 1 1] Revert Hit Material
  (`KismetSystemLibrary.Delay` 0.075)
  (`PrimitiveComponent.SetMaterial` (`self.Mesh`) 0 "/Game/StylizedArmyPackA/materials/M_soldier_body_germany.M_soldier_body_germany")
  (`PrimitiveComponent.SetMaterial` (`self.Default Rifle`) 0 "/Game/StylizedArmyPackA/materials/M_Lion.M_Lion")
  (`PrimitiveComponent.SetMaterial` (`self.SM_soldier_bottle_russia`) 0 "/Game/StylizedArmyPackA/materials/M_soldier_bottle_russia.M_soldier_bottle_russia")
  (`PrimitiveComponent.SetMaterial` (`self.Gas_Canister1`) 0 "/Game/StylizedArmyPackA/materials/M_mine_A.M_mine_A")
  (`PrimitiveComponent.SetMaterial` (`self.Gas_Canister`) 0 "/Game/StylizedArmyPackA/materials/M_mine_A.M_mine_A")
  (`PrimitiveComponent.SetMaterial` (`self.Helmet`) 0 "/Game/StylizedArmyPackA/materials/M_soldier_helmet_C_germany.M_soldier_helmet_C_germany")
  (`PrimitiveComponent.SetMaterial` (`self.SM_soldier_GAZ_germany`) 0 "/Game/StylizedArmyPackA/materials/M_soldier_GAZ_germany.M_soldier_GAZ_germany"))

(event `Death Effect`
  (bind _mesh (`self.Mesh`))
  ;[1 1 1] Death Smoke
  (`KismetSystemLibrary.Delay` 0.2)
  (`PrimitiveComponent.SetCollisionEnabled` (`self.CapsuleComponent`) "NoCollision")
  (`PrimitiveComponent.SetCollisionProfileName` _mesh "Ragdoll" true)
  (`PrimitiveComponent.SetSimulatePhysics` _mesh true)
  (`PrimitiveComponent.AddImpulse` _mesh (0.0 0.0 500.0) "None" false)
  (`CharacterMovementComponent.DisableMovement` (`self.CharacterMovement`))
  (`KismetSystemLibrary.PrintString` "Rifleman Dead")
  (`KismetSystemLibrary.Delay` 3.5)
  (`GameplayStatics.PlaySoundAtLocation` "/Game/Sounds/SC_Smoke_Poof.SC_Smoke_Poof" (`self.K2_GetActorLocation`) (struct) 1.0 1.0 0.0 null null null null)
  (`ActorComponent.Activate` (`self.NS_Death_Smoke`) false)
  (`KismetSystemLibrary.Delay` 0.3)
  (`SceneComponent.SetHiddenInGame` (`self.Mesh`) true true)
  (`self.Stop Firing`)
  (`KismetSystemLibrary.Delay` 1.0)
  (`self.K2_DestroyActor`))

(event `self.AIPerception.OnTargetPerceptionUpdated`
  (params (Actor :type "Actor Object Reference") (Stimulus :type "AIStimulus Structure"))
  ;[1 1 1] AI Perception
  (`BlackboardComponent.SetValueAsBool` (`AIBlueprintHelperLibrary.GetBlackboard` null) "Can See Player" (`.bSuccessfullySensed` (break `AIStimulus` Stimulus))))

(event `self.ReceiveBeginPlay`
  ;[1 1 1] Face Player on Spawn
  (`self.K2_SetActorRotation` (`KismetMathLibrary.FindLookAtRotation` (`self.K2_GetActorLocation`) (`SceneComponent.K2_GetComponentLocation` (`Character.CapsuleComponent` (`GameplayStatics.GetPlayerCharacter` 0))))))

(event `Reset Firing After Hit`
  ;[1 1 1] Reset Firing After Hit
  (if (`self.Is Shooting`)
    (if (not (`self.Is Dead`))
      (`KismetSystemLibrary.Delay` 1.0)
      (`self.Start Firing`))))

(event `/Game/Blueprints/BPI_Enemy_Hit.Enemy Hit`
  (params (`Hit Location` :type "Vector Structure") (Damage :type "Float (double-precision)"))
  (bind _mesh (`self.Mesh`))
  ;[1 1 1] Enemy Hit
  (`PrimitiveComponent.SetMaterial` (`self.Mesh`) 0 "/Game/Materials/MAT_Enemy_Impact_Inst.MAT_Enemy_Impact_Inst")
  (`PrimitiveComponent.SetMaterial` (`self.Helmet`) 0 "/Game/Materials/MAT_Enemy_Impact_Inst.MAT_Enemy_Impact_Inst")
  (`PrimitiveComponent.SetMaterial` (`self.Default Rifle`) 0 "/Game/Materials/MAT_Enemy_Impact_Inst.MAT_Enemy_Impact_Inst")
  (`PrimitiveComponent.SetMaterial` (`self.SM_soldier_bottle_russia`) 0 "/Game/Materials/MAT_Enemy_Impact_Inst.MAT_Enemy_Impact_Inst")
  (`PrimitiveComponent.SetMaterial` (`self.Gas_Canister1`) 0 "/Game/Materials/MAT_Enemy_Impact_Inst.MAT_Enemy_Impact_Inst")
  (`PrimitiveComponent.SetMaterial` (`self.Gas_Canister`) 0 "/Game/Materials/MAT_Enemy_Impact_Inst.MAT_Enemy_Impact_Inst")
  (`PrimitiveComponent.SetMaterial` (`self.SM_soldier_GAZ_germany`) 0 "/Game/Materials/MAT_Enemy_Impact_Inst.MAT_Enemy_Impact_Inst")
  (`NiagaraFunctionLibrary.SpawnSystemAtLocation` "/Game/VFX/Niagara/NS_Hit_Impact.NS_Hit_Impact" `Hit Location`)
  (set `self.Health` (- (`self.Health`) Damage))
  (`self.Stop Firing`)
  (if (== (`KismetMathLibrary.RandomIntegerInRange` 0 1) 0)
    (`self.PlayAnimMontage` "/Game/Animations/AM_Damage1.AM_Damage1" 1.5)
    (else
      (`self.PlayAnimMontage` "/Game/Animations/AM_Damage2.AM_Damage2" 1.5)))
  (`self.Revert Hit Material`)
  (`self.Reset Firing After Hit`)
  ;[1 1 1] Death
  (if (<= (`self.Health`) 0.0)
    (if (not (`self.Is Dead`))
      (`self.Stop Firing`)
      (set `self.Is Dead` true)
      (set `self.Can Shoot` false)
      (`BlackboardComponent.SetValueAsBool` (`AIBlueprintHelperLibrary.GetBlackboard` null) "Is Dead" true)
      (`CharacterMovementComponent.DisableMovement` (`self.CharacterMovement`))
      (`GameplayStatics.PlaySoundAtLocation` "/Game/Sounds/SC_Enemy_Die.SC_Enemy_Die" `Hit Location` (struct) 1.0 1.0 0.0 null null null null)
      (`PrimitiveComponent.SetCollisionEnabled` (`self.CapsuleComponent`) "NoCollision")
      (`KismetSystemLibrary.Delay` 0.3)
      (`PrimitiveComponent.SetCollisionProfileName` _mesh "Ragdoll" true)
      (`PrimitiveComponent.SetSimulatePhysics` _mesh true)
      (`PrimitiveComponent.AddImpulse` _mesh (0.0 0.0 500.0) "None" false)
      (`KismetSystemLibrary.PrintString` "Flamer Dead")
      (`KismetSystemLibrary.Delay` 3.5)
      (`GameplayStatics.PlaySoundAtLocation` "/Game/Sounds/SC_Smoke_Poof.SC_Smoke_Poof" (`self.K2_GetActorLocation`) (struct) 1.0 1.0 0.0 null null null null)
      (`ActorComponent.Activate` (`self.NS_Death_Smoke`) false)
      (`KismetSystemLibrary.Delay` 0.3)
      (`SceneComponent.SetHiddenInGame` (`self.Mesh`) true true)
      (`KismetSystemLibrary.Delay` 1.0)
      (`self.K2_DestroyActor`))))

(event `/Game/Blueprints/BPI_Enemy_Hit.Player Dead`
  ;[1 1 1] Player Dead
  (set `self.Player Died` true)
  (`self.Stop Firing`)
  (`CharacterMovementComponent.DisableMovement` (`self.CharacterMovement`)))

(event `self.Flamethrower.OnComponentActivated`
  (params (Component :type "ActorComponent Object Reference") (bReset :type Boolean))
  ;[1 1 1] Flamethrower Sounds
)

(fn `UserConstructionScript`)