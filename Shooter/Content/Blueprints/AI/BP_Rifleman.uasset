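; Rifleman enemy AI character that shoots at the player, leading shots by player velocity and distance over bullet speed.
; Detection and too-close overlap volumes set blackboard bools on its AI controller.
; StartFiring and StopFiring control the shoot montage, while FireWeapon spawns the bullet with sound and muzzle flash.
; EnemyHit flashes an impact material and subtracts health; death triggers ragdoll, then a smoke poof before destroying the actor.
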(event `Stop Firing`
  ;[1 1 1] Start/Stop Firing
  (`self.StopAnimMontage` "/Game/Animations/AM_Shoot_Rifleman.AM_Shoot_Rifleman")
  (set `self.Is Shooting` false))

(event `Start Firing`
  ;[1 1 1] Start/Stop Firing
  (set `self.Is Shooting` true)
  (`self.PlayAnimMontage` "/Game/Animations/AM_Shoot_Rifleman.AM_Shoot_Rifleman" (`self.Fire Rate`)))

(event `Fire Weapon`
  (bind _returnvalue (`GameplayStatics.GetPlayerCharacter` 0))
  (bind _muzzle_flash (`self.Muzzle Flash`))
  (bind _returnvalue_2 (`SceneComponent.K2_GetComponentLocation` (`self.Spawner`)))
  ;[1 1 1] Spawn Bullet
  (bind _returnvalue_3 (`|SpawnActorFromClass` "/Game/Blueprints/BP_Enemy_Bullet_Rifle.BP_Enemy_Bullet_Rifle_C" (`KismetMathLibrary.MakeTransform` _returnvalue_2 (`KismetMathLibrary.FindLookAtRotation` _returnvalue_2 (+ (+ (`SceneComponent.K2_GetComponentLocation` (`Character.CapsuleComponent` _returnvalue)) (0.0 0.0 0.0)) (* (`self.GetVelocity` _returnvalue) (/ (`self.GetDistanceTo` _returnvalue) (* (`self.Bullet Speed`) 5.0))))) (0.194709 0.032197 0.032197)) "Undefined" "OverrideRootScale" null null))
  (bind _projectilemovement (`/Game/Blueprints/BP_Enemy_Bullet_Rifle.ProjectileMovement` _returnvalue_3))
  (set `MovementComponent.Velocity` (* (`MovementComponent.Velocity` _projectilemovement) (`self.Bullet Speed`)) _projectilemovement)
  ;[1 1 1] Trigger Muzzle Flash
  (`GameplayStatics.PlaySoundAtLocation` "/Game/Sounds/SC_Rifle_Shot.SC_Rifle_Shot" (`self.K2_GetActorLocation`) (struct) 1.0 1.0 0.0 null null null null)
  (`ActorComponent.Activate` _muzzle_flash false)
  (`KismetSystemLibrary.Delay` 0.3)
  (`ActorComponent.Deactivate` _muzzle_flash))

(event `self.ReceiveTick`
  (params (DeltaSeconds :type "Float (single-precision)"))
  (bind _returnvalue (`GameplayStatics.GetPlayerCharacter` 0))
  (set `self.Predicted Rotation` (`KismetMathLibrary.FindLookAtRotation` (`SceneComponent.K2_GetComponentLocation` (`self.Spawner`)) (+ (+ (`SceneComponent.K2_GetComponentLocation` (`Character.CapsuleComponent` _returnvalue)) (0.0 0.0 0.0)) (* (`self.GetVelocity` _returnvalue) (/ (`self.GetDistanceTo` _returnvalue) (* (`self.Bullet Speed`) 5.0)))))))

(event `self.Player Detection.OnComponentBeginOverlap`
  (params (OverlappedComponent :type "PrimitiveComponent Object Reference") (OtherActor :type "Actor Object Reference") (OtherComp :type "PrimitiveComponent Object Reference") (OtherBodyIndex :type Integer) (bFromSweep :type Boolean) (SweepResult :type "HitResult Structure (by ref)"))
  ;[1 1 1] Player Detection
  (if (not (`self.Is Dead`))
    (cast `/Game/Blueprints/BP_ThirdPersonCharacter` OtherActor)
    (`BlackboardComponent.SetValueAsBool` (`AIBlueprintHelperLibrary.GetBlackboard` (`AIBlueprintHelperLibrary.GetAIController` self)) "Player In Range" true)))

(event `Revert Hit Material`
  ;[1 1 1] Revert Hit Material
  (`KismetSystemLibrary.Delay` 0.075)
  (`PrimitiveComponent.SetMaterial` (`self.Mesh`) 0 "/Game/StylizedArmyPackA/materials/M_soldier_body_germany.M_soldier_body_germany")
  (`PrimitiveComponent.SetMaterial` (`self.Default Rifle`) 0 "/Game/StylizedArmyPackA/materials/M_mouse_rifle.M_mouse_rifle")
  (`PrimitiveComponent.SetMaterial` (`self.Backpack`) 0 "/Game/StylizedArmyPackA/materials/M_soldier_backpack_germany.M_soldier_backpack_germany")
  (`PrimitiveComponent.SetMaterial` (`self.Radio`) 0 "/Game/StylizedArmyPackA/materials/M_radio_russia.M_radio_russia")
  (`PrimitiveComponent.SetMaterial` (`self.Helmet`) 0 "/Game/StylizedArmyPackA/materials/M_soldier_helmet_C_germany.M_soldier_helmet_C_germany"))

(event `self.Player Detection.OnComponentEndOverlap`
  (params (OverlappedComponent :type "PrimitiveComponent Object Reference") (OtherActor :type "Actor Object Reference") (OtherComp :type "PrimitiveComponent Object Reference") (OtherBodyIndex :type Integer))
  ;[1 1 1] Player Detection
  (if (not (`self.Is Dead`))
    (cast `/Game/Blueprints/BP_ThirdPersonCharacter` OtherActor)
    (`BlackboardComponent.SetValueAsBool` (`AIBlueprintHelperLibrary.GetBlackboard` (`AIBlueprintHelperLibrary.GetAIController` self)) "Player In Range" false)))

(event `Death Effect`
  ;[1 1 1] Death Smoke
  (`KismetSystemLibrary.Delay` 3.5)
  (`GameplayStatics.PlaySoundAtLocation` "/Game/Sounds/SC_Smoke_Poof.SC_Smoke_Poof" (`self.K2_GetActorLocation`) (struct) 1.0 1.0 0.0 null null null null)
  (`ActorComponent.Activate` (`self.NS_Death_Smoke`) false)
  (`KismetSystemLibrary.Delay` 0.3)
  (`SceneComponent.SetHiddenInGame` (`self.Mesh`) true true)
  (`KismetSystemLibrary.Delay` 1.0)
  (`self.K2_DestroyActor`))

(event `self.Player Too Close.OnComponentBeginOverlap`
  (params (OverlappedComponent :type "PrimitiveComponent Object Reference") (OtherActor :type "Actor Object Reference") (OtherComp :type "PrimitiveComponent Object Reference") (OtherBodyIndex :type Integer) (bFromSweep :type Boolean) (SweepResult :type "HitResult Structure (by ref)"))
  ;[1 1 1] Check Player Isnt Too close
  (cast `/Game/Blueprints/BP_ThirdPersonCharacter` OtherActor)
  (if (not (`self.Is Dead`))
    (`BlackboardComponent.SetValueAsBool` (`AIBlueprintHelperLibrary.GetBlackboard` (`AIBlueprintHelperLibrary.GetAIController` self)) "Player Too Close" true)))

(event `self.Player Too Close.OnComponentEndOverlap`
  (params (OverlappedComponent :type "PrimitiveComponent Object Reference") (OtherActor :type "Actor Object Reference") (OtherComp :type "PrimitiveComponent Object Reference") (OtherBodyIndex :type Integer))
  ;[1 1 1] Check Player Isnt Too close
  (cast `/Game/Blueprints/BP_ThirdPersonCharacter` OtherActor)
  (if (not (`self.Is Dead`))
    (`BlackboardComponent.SetValueAsBool` (`AIBlueprintHelperLibrary.GetBlackboard` (`AIBlueprintHelperLibrary.GetAIController` self)) "Player Too Close" false)))

(fn `Enemy Hit`
  (params (`Hit Location` :type "Vector Structure") (Damage :type "Float (double-precision)"))
  (bind _mesh (`self.Mesh`))
  (`PrimitiveComponent.SetMaterial` (`self.Mesh`) 0 "/Game/Materials/MAT_Enemy_Impact_Inst.MAT_Enemy_Impact_Inst")
  (`PrimitiveComponent.SetMaterial` (`self.Default Rifle`) 0 "/Game/Materials/MAT_Enemy_Impact_Inst.MAT_Enemy_Impact_Inst")
  (`PrimitiveComponent.SetMaterial` (`self.Backpack`) 0 "/Game/Materials/MAT_Enemy_Impact_Inst.MAT_Enemy_Impact_Inst")
  (`PrimitiveComponent.SetMaterial` (`self.Radio`) 0 "/Game/Materials/MAT_Enemy_Impact_Inst.MAT_Enemy_Impact_Inst")
  (`PrimitiveComponent.SetMaterial` (`self.Helmet`) 0 "/Game/Materials/MAT_Enemy_Impact_Inst.MAT_Enemy_Impact_Inst")
  (`NiagaraFunctionLibrary.SpawnSystemAtLocation` "/Game/VFX/Niagara/NS_Hit_Impact.NS_Hit_Impact" `Hit Location`)
  (set `self.Health` (- (`self.Health`) Damage))
  (`self.Revert Hit Material`)
  (if (<= (`self.Health`) 0.0)
    (set `self.Is Dead` true)
    (`self.Stop Firing`)
    (`GameplayStatics.PlaySoundAtLocation` "/Game/Sounds/SC_Enemy_Die.SC_Enemy_Die" `Hit Location` (struct) 1.0 1.0 0.0 null null null null)
    (`PrimitiveComponent.SetCollisionEnabled` (`self.CapsuleComponent`) "NoCollision")
    (`PrimitiveComponent.SetCollisionProfileName` _mesh "Ragdoll" true)
    (`PrimitiveComponent.SetSimulatePhysics` _mesh true)
    (`PrimitiveComponent.AddImpulse` _mesh (0.0 0.0 500.0) "None" false)
    (`CharacterMovementComponent.DisableMovement` (`self.CharacterMovement`))
    (`KismetSystemLibrary.PrintString` "Dead")
    (`self.Death Effect`)))

(fn `UserConstructionScript`)